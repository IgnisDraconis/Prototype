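; BP_EnergyShield is a damageable energy shield that loses health when hit and regenerates after a delay.
; Damage lowers MinDamage, which serves as current health, hides and disables the mesh at zero, and schedules BeginRecharge after ReloadTime.
; BeginRecharge re-enables the shield and sets IsCharging, whose RepNotify starts a self-rescheduling timer that restores one point per FireRate interval.
; A dynamic material's HealthPercent parameter displays the remaining health.
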(event Custom|DisableShield
  (bind _shieldmesh (Variables|Default|GetShieldMesh))
  (Components|Activation|Deactivate _shieldmesh)
  (Collision|SetCollisionEnabled _shieldmesh "NoCollision")
  (Rendering|SetVisibility _shieldmesh false false))

(event Custom|Initalize
  (params (start%20active :type Boolean))
  (if (not start%20active)
    (CallFunction|DisableShield)))

(event Custom|UpdateShield
  (Rendering|Material|SetScalarParameterValue (stale EventBeginPlay _returnvalue) "HealthPercent" (/ (Math|Conversions|ToFloat(Integer) (Variables|Default|GetminDamage)) (Math|Conversions|ToFloat(Integer) (Variables|Default|GetmaxDamage))) :!class /Script/Engine.MaterialInstanceDynamic))

(event Custom|BeginRecharge
  (CallFunction|EnableShield)
  (Variables|Default|SetisCharging true))

(event Custom|EnableShield
  (bind _shieldmesh (Variables|Default|GetShieldMesh))
  (Components|Activation|Activate _shieldmesh false)
  (Collision|SetCollisionEnabled _shieldmesh "QueryOnly")
  (Rendering|SetVisibility _shieldmesh true false))

(event Custom|RechargeTick
  (if (Variables|Default|GetisCharging)
    (Math|Integer|IncrementInt (Variables|Default|GetminDamage)
      (:%20%20
        (Variables|Default|SetminDamage (Math|Integer|Clamp(Integer) (Variables|Default|GetminDamage) 0 (Variables|Default|GetmaxDamage)))
        (CallFunction|UpdateShield)
        (bind _returnvalue (Utilities|Time|SetTimerbyEvent (delegate Custom|RechargeTick) (Variables|Default|GetfireRate)))))
    (else
      (Utilities|Time|ClearandInvalidateTimerbyHandle _returnvalue))))

(event Custom|HitShield
  (Variables|Default|SetisCharging false)
  (Utilities|Time|SetTimerbyEvent (delegate Custom|BeginRecharge) (Variables|Default|GetreloadTime)))

(event EventBeginPlay
  (CallFunction|Initalize (Variables|Default|GetisStartEnabled))
  (bind _output_get (Variables|Default|SetShieldData (Rendering|Material|GetMaterial (Variables|Default|GetShieldMesh) 0)))
  (bind _returnvalue (Rendering|Material|CreateDynamicMaterialInstance (Variables|Default|GetShieldMesh) 0 _output_get "None" :!class /Script/Engine.PrimitiveComponent))
  (Rendering|Material|SetScalarParameterValue _returnvalue "HealthPercent" (/ (Math|Conversions|ToFloat(Integer) (Variables|Default|GetminDamage)) (Math|Conversions|ToFloat(Integer) (Variables|Default|GetmaxDamage))) :!class /Script/Engine.MaterialInstanceDynamic))

(event Game|Damage|EventAnyDamage
  (params (Damage :type Float%20%28single-precision%29) (DamageType :type Damage%20Type%20Object%20Reference) (InstigatedBy :type Controller%20Object%20Reference) (DamageCauser :type Actor%20Object%20Reference))
  (CallFunction|HitShield)
  (Utilities|DamageMacro Damage))

(fn ConstructionScript
  (|CallParentFunction))

(fn OnRepIsCharging
  (CallFunction|RechargeTick))