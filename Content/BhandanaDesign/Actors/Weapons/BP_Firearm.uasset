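; Firearm weapon actor attached to an RPG_Actor, taking its model, material and projectile settings from that parent's CurrentWeapon data.
; ShootGun forwards to a server shoot event that line-traces between camera points to aim a projectile spawned at the Barrel socket, tagged with the owner's tag.
; Authority rolls damage within the weapon's range and writes it, with damage type, onto the bullet.
; BeginPlay caches the parent, sets ownership and applies appearance; equip hooks are empty.
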(event Custom|RUNONSERVER%20Shoot
  (params (Instigator :type Pawn%20Object%20Reference) (Owner%20Tag :type Name) (Camera%20Forward :type Vector) (Camera%20Forward%202 :type Vector))
  (bind _parentactor (Variables|Default|GetParentActor))
  (bind _currentweapon (Variables|/Game/BhandanaDesign/Actors/RPG_Actor.RPG_Actor_C|GetCurrentWeapon _parentactor))
  (bind (_outhit _returnvalue) (Collision|LineTraceForObjects Camera%20Forward%202 Camera%20Forward (Variables|Default|GetTargets) false (Utilities|Array|MakeArray (Variables|Default|GetParentActor)) "None" true "(R=1.000000,G=0.000000,B=0.000000,A=1.000000)" "(R=0.000000,G=1.000000,B=0.000000,A=1.000000)" 9999.0))
  (bind (_projetile_rotation _firepoint) (Utilities|CalculateBulletPath _outhit _returnvalue (.location (Transformation|GetSocketTransform (Variables|Default|GetModel) "Barrel" "RTS_World")))
    (:%20%20
      (bind _returnvalue_2 (Game|SpawnActorfromClass (.projectile _currentweapon) (Math|Transform|MakeTransform _firepoint _projetile_rotation (.projectilesize _currentweapon)) "Undefined" 0 Instigator))
      (Variables|/Game/BhandanaDesign/Actors/Projectiles/BP_Projectile.BP_Projectile_C|SetTagData _returnvalue_2 Owner%20Tag)
      (Networking|SwitchHasAuthority
        (:Authority
          (bind _output_get (Variables|Default|SetfinalDamage (Math|Random|RandomIntegerinRange (.mindamage _currentweapon) (.maxdamage _currentweapon))))
          (CallFunction|UpdateBulletProperties _output_get (.damagetype _currentweapon) _returnvalue_2))))))

(event Custom|ShootGun
  (params (Instigator :type Pawn%20Object%20Reference) (OwnerTag :type Name) (CameraForward :type Vector) (Camera%20Forward%202 :type Vector))
  (CallFunction|RUNONSERVERShoot Instigator OwnerTag CameraForward Camera%20Forward%202))

(event Custom|UpdateBulletProperties
  (params (FinalDamage :type Integer) (DamageType :type Damage%20Type%20Class%20Reference) (Bullet :type BP%20Projectile%20Object%20Reference))
  (if (Utilities|IsValid Bullet)
    (Variables|/Game/BhandanaDesign/Actors/Projectiles/BP_Projectile.BP_Projectile_C|SetDamage Bullet FinalDamage)
    (Variables|/Game/BhandanaDesign/Actors/Projectiles/BP_Projectile.BP_Projectile_C|SetDamageType Bullet DamageType)))

(event Custom|Multicast%20Initialize
  (params (Owner :type Actor%20Object%20Reference))
  (Actor|SetOwner Owner))

(event Custom|UpdateSmallerData
  (bind _asrpg_actor (Utilities|Casting|CastToRPG_Actor (Actor|GetParentActor)))
  (Variables|Default|SetWeaponData (Variables|/Game/BhandanaDesign/Actors/RPG_Actor.RPG_Actor_C|GetCurrentWeapon _asrpg_actor)))

(event Custom|OnUnequip)

(event Custom|OnEquip)

(event EventBeginPlay
  (bind _returnvalue (Actor|GetParentActor))
  (bind _asrpg_actor (Utilities|Casting|CastToRPG_Actor _returnvalue))
  (Variables|Default|SetParentActor _asrpg_actor)
  (bind _output_get (Variables|Default|SetWeaponData (Variables|/Game/BhandanaDesign/Actors/RPG_Actor.RPG_Actor_C|GetCurrentWeapon _asrpg_actor)))
  (CallFunction|MulticastInitialize _returnvalue)
  (Utilities|UpdateWeaponAppearance (.Model (Utilities|Struct|BreakST_WeaponData _output_get)) (.Material (Utilities|Struct|BreakST_WeaponData _output_get)) self
    (:%20%20
      (CallFunction|OnUnequip))))

(fn ConstructionScript)