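; Dual pistols weapon Blueprint that pairs a main gun with an offhand child actor and alternates shots between them.
; The server shoot event line-traces from the camera, flip-flops between the two Barrel sockets and spawns the current weapon's projectile along the calculated path.
; With authority, each bullet gets random damage and a damage type from the gun that fired it.
; Equip and unequip move the offhand, found by class lookup, between active and inactive mesh sockets.
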(event EventBeginPlay
  (bind _offhand (Variables|Default|GetOffhand))
  (bind _childactor (Variables|/Script/Engine.ChildActorComponent|GetChildActor _offhand))
  (|CallParentFunction)
  (bind _asbp_offhand_weapon (Utilities|Casting|CastToBP_OffhandWeapon _childactor))
  (Transformation|AttachComponentToComponent _childactor (Variables|/Script/Engine.Character|GetMesh (Variables|Default|GetParentActor)) (Variables|/Game/BhandanaDesign/Actors/Weapons/BP_OffhandWeapon.BP_OffhandWeapon_C|GetactiveSocket _asbp_offhand_weapon) "KeepRelative" "KeepRelative" "KeepRelative" true))

(event Collision|EventActorBeginOverlap
  (params (OtherActor :type Actor%20Object%20Reference)))

(event EventTick
  (params (DeltaSeconds :type Float%20%28single-precision%29)))

(event EventRUNONSERVERShoot
  (params (Instigator :type Pawn%20Object%20Reference) (Owner%20Tag :type Name :default "None") (Camera%20Forward :type Vector :default "0, 0, 0") (Camera%20Forward%202 :type Vector :default "0, 0, 0"))
  (bind _parentactor (Variables|Default|GetParentActor))
  (bind _currentweapon (Variables|/Game/BhandanaDesign/Actors/RPG_Actor.RPG_Actor_C|GetCurrentWeapon _parentactor))
  (bind _isa (Utilities|FlowControl|FlipFlop)
    (:A
      _)
    (:B
      _))
  (bind (_outhit _returnvalue) (Collision|LineTraceForObjects Camera%20Forward%202 Camera%20Forward (Variables|Default|GetTargets) false (Utilities|Array|MakeArray (Variables|Default|GetParentActor)) "None" true "(R=1.000000,G=0.000000,B=0.000000,A=1.000000)" "(R=0.000000,G=1.000000,B=0.000000,A=1.000000)" 9999.0))
  (if _isa
    (bind (_projetile_rotation _firepoint) (Utilities|CalculateBulletPath _outhit _returnvalue (.location (Transformation|GetSocketTransform (Variables|Default|GetModel) "Barrel" "RTS_World")))
      (:%20%20
        (bind _returnvalue_2 (Game|SpawnActorfromClass (.projectile _currentweapon) (Math|Transform|MakeTransform _firepoint _projetile_rotation (.projectilesize _currentweapon)) "Undefined" Instigator Instigator))
        (Variables|/Game/BhandanaDesign/Actors/Projectiles/BP_Projectile.BP_Projectile_C|SetTagData _returnvalue_2 Owner%20Tag)
        (Networking|SwitchHasAuthority
          (:Authority
            (bind _output_get (Variables|Default|SetfinalDamage (Math|Random|RandomIntegerinRange (.mindamage _currentweapon) (.maxdamage _currentweapon))))
            (CallFunction|UpdateBulletProperties _output_get (.damagetype _currentweapon) _returnvalue_2)))))
    (else
      (bind _asbp_offhand_weapon (Utilities|Casting|CastToBP_OffhandWeapon (Variables|/Script/Engine.ChildActorComponent|GetChildActor (Variables|Default|GetOffhand))))
      (bind (_projetile_rotation_2 _firepoint_2) (Utilities|CalculateBulletPath _outhit _returnvalue (.location (Transformation|GetSocketTransform (Variables|/Game/BhandanaDesign/Actors/Weapons/BP_OffhandWeapon.BP_OffhandWeapon_C|GetMODEL _asbp_offhand_weapon) "Barrel" "RTS_World")))
        (:%20%20
          (bind _returnvalue_3 (Game|SpawnActorfromClass (.projectile _currentweapon) (Math|Transform|MakeTransform _firepoint_2 _projetile_rotation_2 (.projectilesize _currentweapon)) "Undefined" Instigator Instigator))
          (Variables|/Game/BhandanaDesign/Actors/Projectiles/BP_Projectile.BP_Projectile_C|SetTagData _returnvalue_3 Owner%20Tag)
          (Networking|SwitchHasAuthority
            (:Authority
              (bind _output_get_2 (Variables|Default|SetfinalDamage (Math|Random|RandomIntegerinRange (Variables|/Game/BhandanaDesign/Actors/Weapons/BP_OffhandWeapon.BP_OffhandWeapon_C|GetminDamage _asbp_offhand_weapon) (Variables|/Game/BhandanaDesign/Actors/Weapons/BP_OffhandWeapon.BP_OffhandWeapon_C|GetmaxDamage _asbp_offhand_weapon))))
              (CallFunction|UpdateBulletProperties _output_get_2 (Variables|/Game/BhandanaDesign/Actors/Weapons/BP_OffhandWeapon.BP_OffhandWeapon_C|GetdamageType _asbp_offhand_weapon) _returnvalue_3))))))))

(event EventOnUnequip
  (Utilities|UnequipOffhand))

(event EventOnEquip
  (Utilities|EquipOffhand))

(fn ConstructionScript
  (|CallParentFunction))