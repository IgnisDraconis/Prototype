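; BP_Projectile is a projectile actor that deals damage to tagged entities it hits.
; When its Model component hits an actor tagged Entity that lacks the TagData tag, it applies Damage with the configured DamageType.
; Player controller 0 is always the instigator.
; The projectile then destroys itself through a Cleanup event; other hits leave it in place.
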(event OnComponentHit(Model)
  (params (HitComponent :type Primitive%20Component%20Object%20Reference) (OtherActor :type Actor%20Object%20Reference) (OtherComp :type Primitive%20Component%20Object%20Reference) (NormalImpulse :type Vector :default "0, 0, 0") (Hit :type Hit%20Result%20Structure%20%28by%20ref%29))
  (if (Actor|ActorHasTag OtherActor "Entity")
    (if (not (Actor|ActorHasTag OtherActor (Variables|Default|GetTagData)))
      (Game|Damage|ApplyDamage OtherActor (Math|Conversions|ToFloat(Integer) (Variables|Default|GetDamage)) (Game|GetPlayerController 0) self (Variables|Default|GetDamageType))
      (CallFunction|Cleanup self))))

(event Custom|Cleanup
  (params (ActorToDestory :type Actor%20Object%20Reference))
  ;[1 1 1] Removes Self
  (Actor|DestroyActor ActorToDestory))

(fn ConstructionScript)