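; BP_DummyTarget is a damageable target dummy that shows floating combat text when hit and is destroyed when its health runs out.
; Incoming damage runs through CalculateDamages with its resistances and the damage-type table fetched from BP_GlobalVariables on BeginPlay.
; MulticastCombatText projects a spawn point to screen space for a colored DamageFont widget.
; Death follows a short delay; separate cleanup events destroy a given actor.
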(event Custom|Cleanup
  (params (DeletedActor :type Actor%20Object%20Reference))
  (Actor|DestroyActor DeletedActor))

(event Custom|BeginCleanup
  (params (ActorToDestroy :type Actor%20Object%20Reference))
  (CallFunction|Cleanup ActorToDestroy))

(event Custom|Death
  (Actor|DestroyActor self))

(event Custom|MulticastCombatText
  (params (damage :type Float%20%28single-precision%29) (Font%20Color :type Color%20Structure))
  (bind _returnvalue (UserInterface|CreateWidget "/Game/BhandanaDesign/Widgets/DamageFont.DamageFont_C"))
  (Variables|/Game/BhandanaDesign/Widgets/DamageFont.DamageFont_C|SetScreenLocation2D _returnvalue (.ScreenPosition (Class|GameplayStatics|ProjectWorldtoScreen (Game|GetPlayerController 0) (Transformation|GetWorldLocation (Variables|Default|GetDamageTextSpawnPoint)) false)))
  (UserInterface|Viewport|AddtoViewport _returnvalue 0)
  (Default|AssignDamage _returnvalue damage Font%20Color))

(event EventBeginPlay
  (bind _outactors (Actor|GetAllActorsOfClass "/Game/BhandanaDesign/VariableData/BP_GlobalVariables.BP_GlobalVariables_C"))
  (Variables|Default|SetDamageTypes (Variables|/Game/BhandanaDesign/VariableData/BP_GlobalVariables.BP_GlobalVariables_C|GetDamageTypes (Utilities|Array|Get(acopy) _outactors))))

(event Game|Damage|EventAnyDamage
  (params (Damage :type Float%20%28single-precision%29) (DamageType :type Damage%20Type%20Object%20Reference) (InstigatedBy :type Controller%20Object%20Reference) (DamageCauser :type Actor%20Object%20Reference))
  (bind (_new_health _new_damage _text_color) (Utilities|CalculateDamages Damage DamageType (Variables|Default|GetHealth) (Variables|Default|GetResistances) (Variables|Default|GetDamageTypes))
    (:Alive
      (Variables|Default|SetHealth _new_health)
      (CallFunction|MulticastCombatText _new_damage _text_color))
    (:Dead
      (Variables|Default|SetHealth _new_health)
      (CallFunction|MulticastCombatText _new_damage _text_color)
      (Utilities|FlowControl|Delay 0.1)
      (CallFunction|Death))))

(fn ConstructionScript)